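; Actor that shows 3D text over a backing plane fitted to the text with adjustable margins.
; Text and value change events update the Text3D or one of four margins (left, top, right, bottom), then refit the plane, as does BeginPlay.
; Refitting offsets the plane from the colliding-component bounds origin by half the extrusion and margin differences, then scales it to those bounds plus margins.
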(event `self.ReceiveBeginPlay`
  (`self.ModifyPlane`)
  (add `self.OnTextChanged` (delegate `CustomEvent_0`))
  (add `self.OnValueChanged` (delegate `CustomEvent_1`)))

(event `CustomEvent_0` :!signature `self.OnTextChanged`
  (params (Text :type "Text (by ref)"))
  (`Text3DComponent.SetText` (`self.Text3D`) Text)
  (`self.ModifyPlane`))

(event `CustomEvent_1` :!signature `self.OnValueChanged`
  (params (Value :type "Float (double-precision)") (NewParam :type Integer))
  (`self.ModifyMargin` Value NewParam)
  (`self.ModifyPlane`))

(fn `ModifyMargin`
  (params (Value :type "Float (double-precision)") (ValueType :type Integer))
  (`|VariableSetRef` (select `int` ValueType :`0` (`self.Left`) :`1` (`self.Top`) :`2` (`self.Right`) :`3` (`self.Bottom`)) Value))

(fn `ModifyPlane`
  (`self.SetPlaneLocation`)
  (`self.ResizePlane`))

(fn `ResizePlane`
  (bind (_origin _boxextent) (`self.GetActorBounds` true))
  (bind (_origin_2 _boxextent_2) (`KismetSystemLibrary.GetComponentBounds` (`self.Plane`)))
  (bind (_returnvalue_x _returnvalue_y _returnvalue_z) (`KismetMathLibrary.BreakVector` (* (`SceneComponent.K2_GetComponentScale` (`self.Plane`)) (/ (`KismetMathLibrary.MakeVector` (.x _boxextent) (+ (.y _boxextent) (`self.Left`) (`self.Right`)) (+ (.z _boxextent) (`self.Top`) (`self.Bottom`))) (`KismetMathLibrary.MakeVector` (.x _boxextent_2) (.y _boxextent_2) 50.0)))))
  (`SceneComponent.SetRelativeScale3D` (`self.Plane`) (`KismetMathLibrary.MakeVector` _returnvalue_z _returnvalue_y 1.0)))

(fn `SetPlaneLocation`
  (`SceneComponent.K2_SetWorldLocation` (`self.Plane`) (- (`self.GetActorBounds` true) (`KismetMathLibrary.MakeVector` (/ (`Text3DComponent.Extrude` (`self.Text3D`)) 2.0) (- (`self.Right`) (`self.Left`)) (- (`self.Bottom`) (`self.Top`)))) false false))

(fn `UserConstructionScript`)